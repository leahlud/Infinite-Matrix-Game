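; BP_Enemy is an enemy actor that handles all of its interactions through a single overlap event, with a cast check for each type of actor.
; Touching BP_Player deals EnemyDamage through DecrementHealth and destroys the enemy, while overlapping another BP_Enemy destroys that other enemy.
; A BP_Projectile instigated by the player increases that player's score, then both projectile and enemy are destroyed.
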(event `self.ReceiveActorBeginOverlap`
  (params (OtherActor :type "Actor Object Reference"))
  (`|ExecutionSequence`
    (:`then_0`
      (bind _asbp_player (cast `/Game/InfiniteMatrix/Blueprints/BP_Player` OtherActor))
      (`/Game/InfiniteMatrix/Blueprints/BP_Player.DecrementHealth` _asbp_player (`self.EnemyDamage`))
      (`self.K2_DestroyActor`))
    (:`then_1`
      (bind _asbp_enemy (cast `/Game/InfiniteMatrix/Blueprints/BP_Enemy` OtherActor))
      (`self.K2_DestroyActor` _asbp_enemy))
    (:`then_2`
      (bind _asbp_projectile (cast `/Game/InfiniteMatrix/Blueprints/BP_Projectile` OtherActor))
      (bind _asbp_player_2 (cast `/Game/InfiniteMatrix/Blueprints/BP_Player` (`Actor.Instigator` _asbp_projectile)))
      (`/Game/InfiniteMatrix/Blueprints/BP_Player.IncreaseScore` _asbp_player_2)
      (`self.K2_DestroyActor` _asbp_projectile)
      (`self.K2_DestroyActor`))))

(fn `UserConstructionScript`)